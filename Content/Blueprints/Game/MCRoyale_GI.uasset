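; MCRoyale_GI is a Game Instance Blueprint that shows the game's main menu.
; ShowMainMenu creates the MainMenu_BP widget once, caches it in MainMenuWB for later calls, and adds it to the viewport.
; It then calls ShowUI, which switches the first player controller to UI-only input without mouse lock and shows the cursor.
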(event `ShowMainMenu`
  (`/Engine/EditorBlueprintResources/StandardMacros.IsValid` (`self.MainMenu_WB`)
    (:`Is Valid`
      _)
    (:`Is Not Valid`
      (bind _returnvalue (`|CreateWidget` "/Game/Blueprints/UI/MainMenu_BP.MainMenu_BP_C"))
      (set `self.MainMenu_WB` _returnvalue)))
  (`UserWidget.AddToViewport` (`self.MainMenu_WB`) 0)
  (`self.ShowUI`))