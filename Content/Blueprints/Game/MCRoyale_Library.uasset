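; MCRoyale_Library is a helper library of typed accessor functions for core MCRoyale gameplay objects.
; It casts the current game mode to MCRoyale_GM, the game instance to MCRoyale_GI, and the player character at index 0 to Player_BP.
; Each function returns the cast result and does not continue if the cast fails.
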(fn `Cast_Player_BP`
  (returns (PlayerRef :type "/Game/Blueprints/Player/Player_BP Object Reference"))
  (bind _asplayer_bp (cast `/Game/Blueprints/Player/Player_BP` (`GameplayStatics.GetPlayerCharacter` null)))
  (return _asplayer_bp))

(fn `Cast_Royale_GI`
  (returns (GI_Ref :type "/Game/Blueprints/Game/MCRoyale_GI Object Reference"))
  (bind _asmcroyale_gi (cast `/Game/Blueprints/Game/MCRoyale_GI` (`GameplayStatics.GetGameInstance` null)))
  (return _asmcroyale_gi))

(fn `Cast_Royale_GM`
  (returns (GM_Ref :type "/Game/Blueprints/Game/MCRoyale_GM Object Reference"))
  (bind _asmcroyale_gm (cast `/Game/Blueprints/Game/MCRoyale_GM` (`GameplayStatics.GetGameMode` null)))
  (return _asmcroyale_gm))