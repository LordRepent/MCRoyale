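; Player character Blueprint with left/right movement, a normal jump and a wall jump.
; The MoveRight axis drives movement along the actor's right vector and tracks facing, flipping the mesh by negative Y scale and setting GunArm reverse culling to match.
; Pressing Jump while falling line-traces forward from Arrow1; a wall hit sets velocity to the trace direction mirrored off the impact normal plus an upward boost.
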(event `InputAxis|MoveRight`
  (params (AxisValue :type "Float (single-precision)"))
  (bind _facingleft (`self.FacingLeft`))
  ;[0 1 0] Move Right & Left
  (`self.AddMovementInput` (`self.GetActorRightVector`) AxisValue)
  (if (< AxisValue 0.0)
    (set `self.FacingLeft` true)
    (`SceneComponent.SetWorldScale3D` (`self.Mesh`) (select `bool` _facingleft :`false` (1.75 1.75 1.75) :`true` (1.75 -1.75 1.75) :!type "Vector Structure") :!label _label)
    (`StaticMeshComponent.SetReverseCulling` (`self.GunArm`) _facingleft)
    (elif (> AxisValue 0.0)
      (set `self.FacingLeft` false)
      (goto _label))))

(event `InputAction|Jump`
  (params (Key :type "Key Structure"))
  (bind _arrow1 (`self.Arrow1`))
  (bind _returnvalue (`SceneComponent.K2_GetComponentLocation` _arrow1))
  (bind _returnvalue_2 (+ _returnvalue (* (`SceneComponent.GetForwardVector` _arrow1) 30.0)))
  ;[0 0.2442 1] Normal Jump
  (:`Pressed`
    (if (`NavMovementComponent.IsFalling` (`self.CharacterMovement`))
      ;[0.4386 0 1] Wall Jump
      (bind (_outhit _returnvalue_3) (`KismetSystemLibrary.LineTraceSingle` _returnvalue _returnvalue_2 "TraceTypeQuery4"))
      (if _returnvalue_3
        (set `MovementComponent.Velocity` (+ (* (`KismetMathLibrary.Normal` (`KismetMathLibrary.MirrorVectorByNormal` (- _returnvalue_2 _returnvalue) (`.ImpactNormal` (`GameplayStatics.BreakHitResult` _outhit)))) 350.0) (0.0 0.0 500.0)) (`self.CharacterMovement`)))
      (else
        (`self.Jump`)))))

(fn `UserConstructionScript`)