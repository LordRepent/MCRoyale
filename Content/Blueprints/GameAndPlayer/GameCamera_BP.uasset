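; GameCamera_BP is a shared camera actor that follows the players listed in the Royale game mode's PlayersInGame.
; Each tick it eases toward their middle point with VInterpTo, clamping X between MinX and MaxX.
; GetMiddleOfPlayers uses a lone player's location, passes two players to MidpointOfActors, or with more, pairwise-searches for the furthest-apart pair to pass instead.
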(event `self.ReceiveTick`
  (params (DeltaSeconds :type "Float (single-precision)"))
  (bind _outlocation (`self.GetMiddleOfPlayers`))
  (`self.K2_SetActorLocation` (`KismetMathLibrary.VInterpTo` (`self.K2_GetActorLocation`) (`KismetMathLibrary.MakeVector` (`KismetMathLibrary.FClamp` (.x _outlocation) (`self.MinX`) (`self.MaxX`)) (.y _outlocation) (.z _outlocation)) DeltaSeconds 10.0)))

(fn `GetMiddleOfPlayers`
  (returns (OutLocation :type "Vector Structure"))
  (locals (FurthestPlayerOne :type "/Game/Blueprints/GameAndPlayer/Player_BP Object Reference") (FurthestPlayerTwo :type "/Game/Blueprints/GameAndPlayer/Player_BP Object Reference") (GreatestDistance :type "Float (double-precision)"))
  (bind _playersingame (`/Game/Blueprints/GameInfo/MCRoyale_GM.PlayersInGame` (`/Game/Blueprints/GameInfo/MCRoyale_Library.Cast_Royale_GM`)))
  (bind _output (`|GetArrayItem` _playersingame))
  (if (> (`KismetArrayLibrary.Array_Length` _playersingame) 2)
    (for _array_element _playersingame
      (for _array_element_2 _playersingame
        (bind _returnvalue (`self.GetDistanceTo` _array_element _array_element_2))
        (if (> _returnvalue (`local.GreatestDistance`))
          (set `local.GreatestDistance` _returnvalue)
          (set `local.FurthestPlayerOne` _array_element)
          (set `local.FurthestPlayerTwo` _array_element_2))))
    (return (`self.MidpointOfActors` (`local.FurthestPlayerOne`) (`local.FurthestPlayerTwo`)))
    (elif (== (`KismetArrayLibrary.Array_Length` _playersingame) 1)
      (return (`self.K2_GetActorLocation` _output))
      (else
        (return (`self.MidpointOfActors` _output (`|GetArrayItem` _playersingame 1)))))))

(fn `UserConstructionScript`)