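; MCRoyale game instance Blueprint that manages the main and lobby menus, online sessions and level changes.
; Menu events create and cache their widgets, then call ShowUI for UI-only input with a visible cursor.
; Hosting creates a non-LAN session and opens Lobby as a listen server, while joining takes the first search result.
; OpenNewLevel uses OpenLevel, adding a "servertravel" option string when not standalone.
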(event `HostGame`
  ;[1 0.3054 0] Networking sessions & level travel
  (`CreateSessionCallbackProxy.CreateSession` (`GameplayStatics.GetPlayerController` 0) 4
    (:`OnSuccess`
      (`GameplayStatics.OpenLevel` "Lobby" true "listen"))
    (:`OnFailure`
      (`KismetSystemLibrary.PrintString` "Couldn't host session"))))

(event `ShowMainMenu`
  ;[0 1 0] Show Main Menu Screen
  (`/Engine/EditorBlueprintResources/StandardMacros.IsValid` (`self.MainMenu_WB`)
    (:`Is Valid`
      _)
    (:`Is Not Valid`
      (bind _returnvalue (`|CreateWidget` "/Game/Blueprints/UI/MainMenu_BP.MainMenu_BP_C"))
      (set `self.MainMenu_WB` _returnvalue)))
  (`UserWidget.AddToViewport` (`self.MainMenu_WB`) 0)
  (`self.ShowUI`))

(event `ShowLobbyMenu`
  ;[0 1 0] Show Lobby Menu Screen
  (`/Engine/EditorBlueprintResources/StandardMacros.IsValid` (`self.LobbyMenu_WB`)
    (:`Is Valid`
      _)
    (:`Is Not Valid`
      (bind _returnvalue (`|CreateWidget` "/Game/Blueprints/UI/LobbyMenu_BP.LobbyMenu_BP_C"))
      (set `self.LobbyMenu_WB` _returnvalue)))
  (`UserWidget.AddToViewport` (`self.LobbyMenu_WB`) 0)
  (`self.ShowUI`))

(event `JoinGame`
  (bind _returnvalue (`GameplayStatics.GetPlayerController` 0))
  ;[1 0.3054 0] Networking sessions & level travel
  (bind _results (`FindSessionsCallbackProxy.FindSessions` _returnvalue 100)
    (:`OnSuccess`
      (`JoinSessionCallbackProxy.JoinSession` _returnvalue (`|GetArrayItem` _results)
        (:`OnSuccess`
          (`KismetSystemLibrary.PrintString` "Joined Session"))
        (:`OnFailure`
          (`KismetSystemLibrary.PrintString` "Failed to join session"))))
    (:`OnFailure`
      (`KismetSystemLibrary.PrintString` "Couldn't find session"))))

(event `OpenNewLevel`
  (params (LevelName :type Name))
  ;[1 0.3054 0] Networking sessions & level travel
  (if (`KismetSystemLibrary.IsStandalone`)
    (`GameplayStatics.OpenLevel` LevelName)
    (`KismetSystemLibrary.PrintString` "New Level")
    (else
      (`GameplayStatics.OpenLevel` LevelName true "servertravel")
      (`KismetSystemLibrary.PrintString` "Server New Level"))))