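; MCRoyale_GM is a game mode Blueprint that sets up local multiplayer when play begins in standalone mode.
; It gathers all PlayerStarts, then creates each local player up to NumOfPlayers, spawning controllers only where missing.
; Each Player_BP pawn is recorded in PlayersInGame and moved to the PlayerStart with the matching index.
; It finally spawns a GameCamera_BP at the world origin.
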(event `self.ReceiveBeginPlay`
  (if (`KismetSystemLibrary.IsStandalone`)
    (`self.GetPlayerStarts`)
    (`self.SpawnPlayers`)
    (`|SpawnActorFromClass` "/Game/Blueprints/GameAndPlayer/GameCamera_BP.GameCamera_BP_C" (`KismetMathLibrary.MakeTransform` (0.0 0.0 0.0)) "Undefined" "OverrideRootScale" null null)))

(fn `GetPlayerStarts`
  (bind _outactors (`GameplayStatics.GetAllActorsOfClass` "/Script/Engine.PlayerStart"))
  (set `self.PlayerStarts` _outactors))

(fn `SpawnPlayers`
  (for _index (range (`self.NumOfPlayers`))
    (bind _returnvalue (`GameplayStatics.GetPlayerController` _index))
    (`GameplayStatics.CreatePlayer` _index (select `bool` (`KismetSystemLibrary.IsValid` _returnvalue) :`false` true))
    (bind _asplayer_bp (cast `/Game/Blueprints/GameAndPlayer/Player_BP` (`Controller.K2_GetPawn` _returnvalue)))
    (`KismetArrayLibrary.Array_Add` (`self.PlayersInGame`) _asplayer_bp)
    (`self.K2_SetActorLocation` _asplayer_bp (`self.K2_GetActorLocation` (`|GetArrayItem` (`self.PlayerStarts`) _index)) false false)))

(fn `UserConstructionScript`)